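; BP_task01_Character is a character Blueprint that adds a HUD and shows an interaction widget on the focused target.
; BeginPlay creates W_HUD for the first player controller and adds it to the viewport.
; Each Tick casts FocuseActor, which this graph only reads, to BP_task01_Target, caching it in TempActor and showing its ItteractWidget.
; When the cast fails, it hides the widget on the cached target.
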(event `self.ReceiveBeginPlay`
  (bind _returnvalue (`|CreateWidget` "/Game/Task_01/Widgets/W_HUD.W_HUD_C" (`GameplayStatics.GetPlayerController` 0)))
  (`UserWidget.AddToViewport` _returnvalue 0))

(event `self.ReceiveTick`
  (params (DeltaSeconds :type "Float (single-precision)"))
  (bind _asbp_task_01_target (cast `/Game/Task_01/BP_From_C++/BP_task01_Target` (`self.FocuseActor`))
    (:`then`
      (set `self.Temp Actor` _asbp_task_01_target)
      (`SceneComponent.SetVisibility` (`/Game/Task_01/BP_From_C++/BP_task01_Target.Itteract Widget` _asbp_task_01_target) true false))
    (:`CastFailed`
      (if (!= (`self.Temp Actor`) null)
        (`SceneComponent.SetVisibility` (`/Game/Task_01/BP_From_C++/BP_task01_Target.Itteract Widget` (`self.Temp Actor`)) false false)))))

(fn `UserConstructionScript`)