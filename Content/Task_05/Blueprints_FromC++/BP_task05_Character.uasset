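; BP_task05_Character is a character that moves automatically in a loop along the spline of a BP_Trajectory actor found at BeginPlay.
; Each Tick advances the distance by CurrentSpeed times delta time and sets the capsule's relative transform from the spline's world-space location and rotation, with Z fixed.
; The distance resets to zero once it exceeds the spline length.
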(event `self.ReceiveBeginPlay`
  (bind _returnvalue (`GameplayStatics.GetActorOfClass` "/Game/Task_05/BP_Trajectory.BP_Trajectory_C"))
  (set `self.Spline to walk` _returnvalue))

(event `self.ReceiveTick`
  (params (DeltaSeconds :type "Float (single-precision)"))
  (bind _spline_distance (`self.Spline Distance`))
  (bind (_returnvalue_location _returnvalue_rotation) (`KismetMathLibrary.BreakTransform` (`SplineComponent.GetTransformAtDistanceAlongSpline` (`/Game/Task_05/BP_Trajectory.Spline` (`self.Spline to walk`)) _spline_distance "World" false)))
  (set `self.Spline Distance` (+ (* DeltaSeconds (`self.CurrentSpeed`)) _spline_distance))
  (`SceneComponent.K2_SetRelativeTransform` (`self.CapsuleComponent`) (`KismetMathLibrary.MakeTransform` (`KismetMathLibrary.MakeVector` (.x _returnvalue_location) (.y _returnvalue_location) 100.0) _returnvalue_rotation (`self.GetActorRelativeScale3D` self)) false false)
  (if (> (`self.Spline Distance`) (`SplineComponent.GetSplineLength` (`/Game/Task_05/BP_Trajectory.Spline` (`self.Spline to walk`))))
    (set `self.Spline Distance` 0.0)))

(fn `UserConstructionScript`)